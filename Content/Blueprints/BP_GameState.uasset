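; BP_GameState is the game state that resolves the end of a networked team match and shows the results.
; OnVictory loops PlayerArray, telling Blue avatars they lost and Red avatars they won, then calls ShowResultScreen.
; That function adds a W_GameResults widget showing a loss message to a local Blue player, otherwise the WinningPlayer's nickname as winner.
; Outcomes are hardcoded by team, and OnRestart is empty.
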(event `self.OnVictory`
  (for _array_element (`self.PlayerArray`)
    (bind _asnet_player_state (cast `NetPlayerState` _array_element))
    (bind (_data_nickname _data_customizationdata _data_teamid) (break `SPlayerInfo` (`NetPlayerState.Data` _asnet_player_state)))
    (switch `EPlayerTeam` _data_teamid
      (:`TEAM_Blue`
        (bind _asbp_avatar (cast `/Game/Blueprints/BP_Avatar` (`PlayerState.PawnPrivate` _array_element) :!pure true))
        (`/Game/Blueprints/BP_Avatar.OnPlayerLost` _asbp_avatar))
      (:`TEAM_Red`
        (`/Game/Blueprints/BP_Avatar.OnPlayerWon` _asbp_avatar))))
  (`self.ShowResultScreen`))

(event `self.OnRestart`)

(fn `ShowResultScreen`
  (bind (_data_nickname _data_customizationdata _data_teamid) (break `SPlayerInfo` (`NetPlayerState.Data` (cast `NetPlayerState` (`Controller.PlayerState` (`GameplayStatics.GetPlayerController` 0)) :!pure true))))
  (bind _returnvalue (`self.GetPlayerStateByIndex` (`self.WinningPlayer`)))
  (bind _returnvalue_2 (`|CreateWidget` "/Game/Blueprints/UMG/W_GameResults.W_GameResults_C" null (`KismetMathLibrary.SelectText` "YOU LOSE!" (`|FormatText` "{P} WINS!" (`.NickName` (break `SPlayerInfo` (`NetPlayerState.Data` _returnvalue)))) (`|EnumEquality` _data_teamid "TEAM_Blue"))))
  (bind _output_get (set `self.MessageWidget` _returnvalue_2))
  (`UserWidget.AddToViewport` _output_get 0))

(fn `UserConstructionScript`)